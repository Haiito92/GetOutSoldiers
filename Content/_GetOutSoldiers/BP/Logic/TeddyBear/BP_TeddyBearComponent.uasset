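; Actor component for the teddy bear that plays a voice or sound cue when the player presses its command inputs.
; Enhanced Input actions for movement directions, jump and extra commands like BestFriend, Looser and Youpi each pass an action name to PlayTeddyBearSound.
; That function looks the name up as a row in DT_TeddyBear_Buttons and plays the row's sound as non-spatial 2D audio.
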(event `EnhancedInput|/Game/_GetOutSoldiers/Assets/Inputs/Actions/TeddyBear/IA_Teddy_Backward`
  (params (ActionValue :type Boolean) (ElapsedSeconds :type "Float (double-precision)") (TriggeredSeconds :type "Float (double-precision)") (InputAction :type "InputAction Object Reference" :default "/Game/_GetOutSoldiers/Assets/Inputs/Actions/TeddyBear/IA_Teddy_Backward.IA_Teddy_Backward"))
  ;[1 1 1] Comment
  (:`Started`
    (`self.PlayTeddyBearSound` "Backward")))

(event `EnhancedInput|/Game/_GetOutSoldiers/Assets/Inputs/Actions/TeddyBear/IA_Teddy_Left`
  (params (ActionValue :type Boolean) (ElapsedSeconds :type "Float (double-precision)") (TriggeredSeconds :type "Float (double-precision)") (InputAction :type "InputAction Object Reference" :default "/Game/_GetOutSoldiers/Assets/Inputs/Actions/TeddyBear/IA_Teddy_Left.IA_Teddy_Left"))
  ;[1 1 1] Comment
  (:`Started`
    (`self.PlayTeddyBearSound` "Left")))

(event `EnhancedInput|/Game/_GetOutSoldiers/Assets/Inputs/Actions/TeddyBear/IA_Teddy_Forward`
  (params (ActionValue :type Boolean) (ElapsedSeconds :type "Float (double-precision)") (TriggeredSeconds :type "Float (double-precision)") (InputAction :type "InputAction Object Reference" :default "/Game/_GetOutSoldiers/Assets/Inputs/Actions/TeddyBear/IA_Teddy_Forward.IA_Teddy_Forward"))
  ;[1 1 1] Comment
  (:`Started`
    (`self.PlayTeddyBearSound` "Forward")))

(event `EnhancedInput|/Game/_GetOutSoldiers/Assets/Inputs/Actions/TeddyBear/IA_Teddy_Right`
  (params (ActionValue :type Boolean) (ElapsedSeconds :type "Float (double-precision)") (TriggeredSeconds :type "Float (double-precision)") (InputAction :type "InputAction Object Reference" :default "/Game/_GetOutSoldiers/Assets/Inputs/Actions/TeddyBear/IA_Teddy_Right.IA_Teddy_Right"))
  ;[1 1 1] Comment
  (:`Started`
    (`self.PlayTeddyBearSound` "Right")))

(event `EnhancedInput|/Game/_GetOutSoldiers/Assets/Inputs/Actions/TeddyBear/IA_Teddy_Jump`
  (params (ActionValue :type Boolean) (ElapsedSeconds :type "Float (double-precision)") (TriggeredSeconds :type "Float (double-precision)") (InputAction :type "InputAction Object Reference" :default "/Game/_GetOutSoldiers/Assets/Inputs/Actions/TeddyBear/IA_Teddy_Jump.IA_Teddy_Jump"))
  ;[1 1 1] Comment
  (:`Started`
    (`self.PlayTeddyBearSound` "Jump")))

(event `EnhancedInput|/Game/_GetOutSoldiers/Assets/Inputs/Actions/TeddyBear/IA_Teddy_BFF`
  (params (ActionValue :type Boolean) (ElapsedSeconds :type "Float (double-precision)") (TriggeredSeconds :type "Float (double-precision)") (InputAction :type "InputAction Object Reference" :default "/Game/_GetOutSoldiers/Assets/Inputs/Actions/TeddyBear/IA_Teddy_BFF.IA_Teddy_BFF"))
  ;[1 1 1] Other Commands
  (:`Started`
    (`self.PlayTeddyBearSound` "BestFriend")))

(event `EnhancedInput|/Game/_GetOutSoldiers/Assets/Inputs/Actions/TeddyBear/IA_Teddy_Looser`
  (params (ActionValue :type Boolean) (ElapsedSeconds :type "Float (double-precision)") (TriggeredSeconds :type "Float (double-precision)") (InputAction :type "InputAction Object Reference" :default "/Game/_GetOutSoldiers/Assets/Inputs/Actions/TeddyBear/IA_Teddy_Looser.IA_Teddy_Looser"))
  ;[1 1 1] Other Commands
  (:`Triggered`
    (`self.PlayTeddyBearSound` "Looser")))

(event `EnhancedInput|/Game/_GetOutSoldiers/Assets/Inputs/Actions/TeddyBear/IA_Teddy_Youpi`
  (params (ActionValue :type Boolean) (ElapsedSeconds :type "Float (double-precision)") (TriggeredSeconds :type "Float (double-precision)") (InputAction :type "InputAction Object Reference" :default "/Game/_GetOutSoldiers/Assets/Inputs/Actions/TeddyBear/IA_Teddy_Youpi.IA_Teddy_Youpi"))
  ;[1 1 1] Other Commands
  (:`Started`
    (`self.PlayTeddyBearSound` "Youpi")))

(fn `PlayTeddyBearSound`
  (params (Action :type Name))
  (bind _returnvalue (`|GetDataTableRow` "/Game/_GetOutSoldiers/Assets/Data/DT_TeddyBear_Buttons.DT_TeddyBear_Buttons" Action)
    (:`then`
      (`GameplayStatics.PlaySound2D` (break `/Game/_GetOutSoldiers/BP/Logic/TeddyBear/ST_TeddyBear` _returnvalue) 1.0 1.0 0.0 null null))))