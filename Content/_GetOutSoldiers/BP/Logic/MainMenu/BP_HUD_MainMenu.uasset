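; Main menu HUD that creates and switches between the main, options, high score and level selection screens for the driver player.
; InitHUD builds all widgets upfront, binds their events and gives the no-input player a separate waiting canvas.
; Handlers swap widgets, update the current interaction widget, and relay level selection and quit through dispatchers.
; The high score back handler removes the options widget rather than the high score one.
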(event `self.ReceiveInitHUD`
  (params (InDriverPlayerController :type "GoSPlayerController Object Reference") (InNoInputPlayerController :type "NoInputPlayerController Object Reference"))
  ;[1 1 1] Create Main Menu
  (`|ExecutionSequence`
    (:`then_0`
      (bind _returnvalue (`|CreateWidget` "/Game/_GetOutSoldiers/BP/UI/MainMenu/WBP_MainMenuCanvas.WBP_MainMenuCanvas_C" InDriverPlayerController))
      (bind _output_get (set `self.WBP_MainMenu` _returnvalue))
      (`self.SetCurrentInteractionWidget` _output_get)
      ;[1 1 1] Bind to main menu events
      (add `/Game/_GetOutSoldiers/BP/UI/MainMenu/WBP_MainMenuCanvas.PlayButtonClicked` _output_get (`|CreateDelegate` :!event `OnPlayButtonClicked`))
      (add `/Game/_GetOutSoldiers/BP/UI/MainMenu/WBP_MainMenuCanvas.OptionButtonClicked` _output_get (`|CreateDelegate` :!event `OnOptionButtonClicked`))
      (add `/Game/_GetOutSoldiers/BP/UI/MainMenu/WBP_MainMenuCanvas.QuitButtonClicked` _output_get (`|CreateDelegate` :!event `OnQuitGameClicked`))
      (add `/Game/_GetOutSoldiers/BP/UI/MainMenu/WBP_MainMenuCanvas.HighScoreClicked` _output_get (`|CreateDelegate` :!event `OnHighScoreButtonPressed`))
      ;[1 1 1] Add Main Menu to Viewport
      (`UserWidget.AddToPlayerScreen` (`self.WBP_MainMenu`) 0))
    (:`then_1`
      (bind _returnvalue_2 (`|CreateWidget` "/Game/_GetOutSoldiers/BP/UI/MainMenu/WBP_OptionsMenu.WBP_OptionsMenu_C" InDriverPlayerController))
      (bind _output_get_2 (set `self.WBP_Option` _returnvalue_2))
      (`/Game/_GetOutSoldiers/BP/UI/MainMenu/WBP_OptionsMenu.InitOptions` _output_get_2)
      (add `/Game/_GetOutSoldiers/BP/UI/MainMenu/WBP_OptionsMenu.OnBackClicked` _output_get_2 (`|CreateDelegate` :!event `CE_OnOptionBackButtonPressed`)))
    (:`then_2`
      (bind _returnvalue_3 (`|CreateWidget` "/Game/_GetOutSoldiers/BP/UI/MainMenu/WBP_HighScores.WBP_HighScores_C" InDriverPlayerController))
      (bind _output_get_3 (set `self.WBP_Highscore` _returnvalue_3))
      (`/Game/_GetOutSoldiers/BP/UI/MainMenu/WBP_HighScores.InitHighScoresUI` _output_get_3)
      (add `/Game/_GetOutSoldiers/BP/UI/MainMenu/WBP_HighScores.BackButtonClicked` _output_get_3 (`|CreateDelegate` :!event `OnHighScoreBackButtonPressed`)))
    (:`then_3`
      (bind _returnvalue_4 (`|CreateWidget` "/Game/_GetOutSoldiers/BP/UI/MainMenu/WBP_WaitingCanvas.WBP_WaitingCanvas_C" InNoInputPlayerController))
      (bind _output_get_4 (set `self.WBP_WaintingCanvas` _returnvalue_4))
      (`/Game/_GetOutSoldiers/BP/UI/MainMenu/WBP_WaitingCanvas.InitWaitingCanvas` _output_get_4)
      (`UserWidget.AddToPlayerScreen` _output_get_4 0))
    (:`then_4`
      (bind _returnvalue_5 (`|CreateWidget` "/Game/_GetOutSoldiers/BP/UI/MainMenu/LevelSelection/WBP_LevelSelectionMenu.WBP_LevelSelectionMenu_C" InDriverPlayerController))
      (bind _output_get_5 (set `self.WBP_LevelSelectionMenu` _returnvalue_5))
      (`/Game/_GetOutSoldiers/BP/UI/MainMenu/LevelSelection/WBP_LevelSelectionMenu.InitLevelSelectionMenu` _output_get_5)
      (add `/Game/_GetOutSoldiers/BP/UI/MainMenu/LevelSelection/WBP_LevelSelectionMenu.LevelSelected` _output_get_5 (`|CreateDelegate` :!event `OnLevelSelected`)))))

(event `OnQuitGameClicked`
  ;[1 1 1] On Quit Game Clicked
  (`self.QuitClicked`))

(event `OnLevelSelected`
  (params (GetOutLevelIndex :type Integer))
  ;[1 1 1] On Play Button Clicked
  (`self.LevelSelected` GetOutLevelIndex))

(event `OnOptionButtonClicked`
  (bind _wbp_option (`self.WBP_Option`))
  (`Widget.RemoveFromParent` (`self.WBP_MainMenu`))
  (`UserWidget.AddToPlayerScreen` _wbp_option 0)
  (`self.SetCurrentInteractionWidget` _wbp_option))

(event `CE_OnOptionBackButtonPressed`
  (bind _wbp_mainmenu (`self.WBP_MainMenu`))
  (`Widget.RemoveFromParent` (`self.WBP_Option`))
  (`UserWidget.AddToPlayerScreen` _wbp_mainmenu 0)
  (`self.SetCurrentInteractionWidget` _wbp_mainmenu))

(event `OnHighScoreBackButtonPressed`
  (bind _wbp_mainmenu (`self.WBP_MainMenu`))
  (`Widget.RemoveFromParent` (`self.WBP_Option`))
  (`UserWidget.AddToPlayerScreen` _wbp_mainmenu 0)
  (`self.SetCurrentInteractionWidget` _wbp_mainmenu))

(event `OnHighScoreButtonPressed`
  (bind _wbp_highscore (`self.WBP_Highscore`))
  (`Widget.RemoveFromParent` (`self.WBP_MainMenu`))
  (`UserWidget.AddToPlayerScreen` _wbp_highscore 0)
  (`self.SetCurrentInteractionWidget` _wbp_highscore))

(event `OnPlayButtonClicked`
  (bind _wbp_levelselectionmenu (`self.WBP_LevelSelectionMenu`))
  (`Widget.RemoveFromParent` (`self.WBP_MainMenu`))
  (`UserWidget.AddToPlayerScreen` _wbp_levelselectionmenu 0)
  (`self.SetCurrentInteractionWidget` _wbp_levelselectionmenu))

(fn `UserConstructionScript`)