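; Main menu player controller that turns Enhanced Input actions into menu navigation events.
; On BeginPlay it adds the IMC_Menu mapping context to the local player's Enhanced Input subsystem.
; The Started trigger of the interact and four directional actions each calls the OnMenuInputActionPressed dispatcher with a matching action value, so listeners handle the menu response.
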(event `self.ReceiveBeginPlay`
  (`EnhancedInputSubsystemInterface.AddMappingContext` (subsystem `EnhancedInputLocalPlayerSubsystem`) "/Game/_GetOutSoldiers/Assets/Inputs/IMC_Menu.IMC_Menu" 0 (struct)))

(event `EnhancedInput|/Game/_GetOutSoldiers/Assets/Inputs/Actions/Menu/IA_Interact`
  (params (ActionValue :type Boolean) (ElapsedSeconds :type "Float (double-precision)") (TriggeredSeconds :type "Float (double-precision)") (InputAction :type "InputAction Object Reference" :default "/Game/_GetOutSoldiers/Assets/Inputs/Actions/Menu/IA_Interact.IA_Interact"))
  ;[1 1 1] MenuActions
  (:`Started`
    (`GoSPlayerController.OnMenuInputActionPressed` "Interact")))

(event `EnhancedInput|/Game/_GetOutSoldiers/Assets/Inputs/Actions/Menu/IA_MenuRight`
  (params (ActionValue :type Boolean) (ElapsedSeconds :type "Float (double-precision)") (TriggeredSeconds :type "Float (double-precision)") (InputAction :type "InputAction Object Reference" :default "/Game/_GetOutSoldiers/Assets/Inputs/Actions/Menu/IA_MenuRight.IA_MenuRight"))
  ;[1 1 1] MenuActions
  (:`Started`
    (`GoSPlayerController.OnMenuInputActionPressed` "GoRight")))

(event `EnhancedInput|/Game/_GetOutSoldiers/Assets/Inputs/Actions/Menu/IA_MenuUp`
  (params (ActionValue :type Boolean) (ElapsedSeconds :type "Float (double-precision)") (TriggeredSeconds :type "Float (double-precision)") (InputAction :type "InputAction Object Reference" :default "/Game/_GetOutSoldiers/Assets/Inputs/Actions/Menu/IA_MenuUp.IA_MenuUp"))
  ;[1 1 1] MenuActions
  (:`Started`
    (`GoSPlayerController.OnMenuInputActionPressed` "GoUp")))

(event `EnhancedInput|/Game/_GetOutSoldiers/Assets/Inputs/Actions/Menu/IA_MenuLeft`
  (params (ActionValue :type Boolean) (ElapsedSeconds :type "Float (double-precision)") (TriggeredSeconds :type "Float (double-precision)") (InputAction :type "InputAction Object Reference" :default "/Game/_GetOutSoldiers/Assets/Inputs/Actions/Menu/IA_MenuLeft.IA_MenuLeft"))
  ;[1 1 1] MenuActions
  (:`Started`
    (`GoSPlayerController.OnMenuInputActionPressed` "GoLeft")))

(event `EnhancedInput|/Game/_GetOutSoldiers/Assets/Inputs/Actions/Menu/IA_MenuDown`
  (params (ActionValue :type Boolean) (ElapsedSeconds :type "Float (double-precision)") (TriggeredSeconds :type "Float (double-precision)") (InputAction :type "InputAction Object Reference" :default "/Game/_GetOutSoldiers/Assets/Inputs/Actions/Menu/IA_MenuDown.IA_MenuDown"))
  ;[1 1 1] MenuActions
  (:`Started`
    (`GoSPlayerController.OnMenuInputActionPressed` "GoDown")))

(fn `UserConstructionScript`)