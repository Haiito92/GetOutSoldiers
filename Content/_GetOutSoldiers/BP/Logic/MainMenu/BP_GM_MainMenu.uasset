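; Main menu game mode for GetOutSoldiers that connects the menu HUD's buttons to game actions.
; On InitializeGame it caches the game instance and the main menu HUD, binds to the HUD's Play and Quit click events, and prints an error if either cast fails.
; Play loads Level_Light through the game instance, and Quit exits the game.
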(event `self.ReceiveInitializeGame`
  (bind _hud_mainmenu (`self.HUD_MainMenu`))
  ;[1 1 1] Get GI
  (bind _asgi_get_out_soldiers (cast `/Game/_GetOutSoldiers/BP/Logic/GI_GetOutSoldiers` (`GameplayStatics.GetGameInstance`))
    (:`then`
      (set `self.GameInstance` _asgi_get_out_soldiers)
      ;[1 1 1] Init HUD
      (bind _asbp_hud_main_menu (cast `/Game/_GetOutSoldiers/BP/Logic/MainMenu/BP_HUD_MainMenu` (`PlayerController.GetHUD` (`self.m_DriverPlayerController`)))
        (:`then`
          (set `self.HUD_MainMenu` _asbp_hud_main_menu)
          ;[1 1 1] Bind To HUD Events
          (add `/Game/_GetOutSoldiers/BP/Logic/MainMenu/BP_HUD_MainMenu.PlayClicked` _hud_mainmenu (`|CreateDelegate` :!event `CE_OnHUDPlayClicked`))
          (add `/Game/_GetOutSoldiers/BP/Logic/MainMenu/BP_HUD_MainMenu.QuitClicked` _hud_mainmenu (`|CreateDelegate` :!event `CE_OnQuitGame`)))
        (:`CastFailed`
          (`KismetSystemLibrary.PrintString` "Couldn't get HUDMainMenu" true true (struct :`R` 1.0 :`G` 0.017487 :`A` 1.0) 2.0 "None"))))
    (:`CastFailed`
      (`KismetSystemLibrary.PrintString` "Couldn't get GI_GetOutSoldiers" true true (struct :`R` 1.0 :`G` 0.017487 :`A` 1.0) 2.0 "None"))))

(event `CE_OnHUDPlayClicked`
  (`self.Play`))

(event `CE_OnQuitGame`
  (`KismetSystemLibrary.QuitGame` null "Quit"))

(fn `Play`
  (`/Game/_GetOutSoldiers/BP/Logic/GI_GetOutSoldiers.LoadLevel` (`self.GameInstance`) "Level_Light"))

(fn `UserConstructionScript`)