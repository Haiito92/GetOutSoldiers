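; Camera controller component that drives a camera actor from the average transform of all currently active views.
; InitCameraController binds to each view's activation event to maintain ActiveViews, then makes the camera the player's view target.
; Each tick averages view locations and raw Euler rotations into a target, then moves the camera halfway toward it, giving frame-rate-dependent smoothing.
; With no active views, the target falls back to a default transform.
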(event `self.ReceiveTick`
  (params (DeltaSeconds :type "Float (single-precision)"))
  (bind _computedconfiguration (`self.Compute Average Configuration`))
  (set `self.TargetConfiguration` _computedconfiguration)
  (`self.LerpCurrentConfiguration`)
  (`self.ApplyCurrentConfiguration`))

(event `CE_OnViewActivationStateChanged`
  (params (View :type "/Game/_GetOutSoldiers/BP/Logic/Camera/Views/BP_AView Object Reference") (IsActivated :type Boolean))
  (if IsActivated
    (`self.AddActiveView` View)
    (else
      (`self.RemoveActiveView` View))))

(fn `AddActiveView`
  (params (AddedView :type "/Game/_GetOutSoldiers/BP/Logic/Camera/Views/BP_AView Object Reference"))
  (`KismetArrayLibrary.Array_AddUnique` (`self.ActiveViews`) AddedView))

(fn `ApplyCurrentConfiguration`
  (`Actor.K2_SetActorTransform` (`self.Camera`) (`self.CurrentConfiguration`) false false))

(fn `Compute Average Configuration`
  (returns (ComputedConfiguration :type "Transform Structure"))
  (locals (AverageConfiguration :type "Transform Structure"))
  (bind _averageconfiguration (`local.AverageConfiguration`))
  (bind _averageconfiguration_2 (`local.AverageConfiguration`))
  (bind _returnvalue (`KismetArrayLibrary.Array_Length` (`self.ActiveViews`)))
  (set `local.AverageConfiguration` (struct))
  (if (== (`KismetArrayLibrary.Array_Length` (`self.ActiveViews`)) 0)
    (return (`local.AverageConfiguration`))
    (else
      (for _array_element (`self.ActiveViews`)
        (bind _viewconfiguration (`/Game/_GetOutSoldiers/BP/Logic/Camera/Views/BP_AView.GetConfiguration` _array_element))
        ;[1 1 1] Add to average Config (except Yaw)
        (set `local.AverageConfiguration` (`KismetMathLibrary.MakeTransform` (+ (.location _averageconfiguration_2) (.location _viewconfiguration)) (`KismetMathLibrary.MakeRotator` (+ (.roll (.rotation _viewconfiguration)) (.roll (.rotation _averageconfiguration_2))) (+ (.pitch (.rotation _viewconfiguration)) (.pitch (.rotation _averageconfiguration_2))) (+ (.yaw (.rotation _viewconfiguration)) (.yaw (.rotation _averageconfiguration_2)))))))
      (bind _output_get (set `local.AverageConfiguration` (`KismetMathLibrary.MakeTransform` (/ (.location _averageconfiguration) _returnvalue) (`KismetMathLibrary.MakeRotator` (/ (.roll (.rotation _averageconfiguration)) _returnvalue) (/ (.pitch (.rotation _averageconfiguration)) _returnvalue) (/ (.yaw (.rotation _averageconfiguration)) _returnvalue)))))
      (return _output_get))))

(fn `InitCameraController`
  (params (Views :type "Array of /Game/_GetOutSoldiers/BP/Logic/Camera/Views/BP_AView Object Reference") (PlayerController :type "PlayerController Object Reference"))
  (`|ExecutionSequence`
    (:`then_0`
      ;[1 1 1] Bind to views events
      (for _array_element Views
        (add `/Game/_GetOutSoldiers/BP/Logic/Camera/Views/BP_AView.ActivationStateUpdated` _array_element (`|CreateDelegate` :!event `CE_OnViewActivationStateChanged`))
        (`/Game/_GetOutSoldiers/BP/Logic/Camera/Views/BP_AView.InitView` _array_element)))
    (:`then_1`
      (bind _computedconfiguration (`self.Compute Average Configuration`))
      (set `self.TargetConfiguration` _computedconfiguration)
      (`PlayerController.SetViewTargetWithBlend` PlayerController (`self.Camera`) 0.0 "VTBlend_Linear" 0.0 false))))

(fn `LerpCurrentConfiguration`
  (set `self.CurrentConfiguration` (`KismetMathLibrary.TLerp` (`self.CurrentConfiguration`) (`self.TargetConfiguration`) 0.5)))

(fn `RemoveActiveView`
  (params (RemovedView :type "/Game/_GetOutSoldiers/BP/Logic/Camera/Views/BP_AView Object Reference"))
  (`KismetArrayLibrary.Array_RemoveItem` (`self.ActiveViews`) RemovedView))