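; View volume blender component that tracks active camera view volumes and the views they reference.
; InitViewVolumeBlender assigns each volume a unique ID and binds its activation event to add or remove it from the active list.
; A view-to-volume map stores the first volume added per view and switches that view active; removal drops the view's entry without deactivating it.
; Tick only resets mapped views' weights to zero, with no blend calculation.
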(event `self.ReceiveTick`
  (params (DeltaSeconds :type "Float (single-precision)"))
  (bind _keys (`BlueprintMapLibrary.Map_Keys` (`self.VolumesPerView`)))
  (for _array_element _keys
    (set `/Game/_GetOutSoldiers/BP/Logic/Camera/Views/BP_AView.Weight` 0.0 _array_element)))

(event `CE_OnViewVolumeActivationStateUpdated`
  (params (ViewVolume :type "/Game/_GetOutSoldiers/BP/Logic/Camera/Volumes/BP_AViewVolume Object Reference") (IsActive :type Boolean))
  ;[1 1 1] React to View Volumes Events
  (if IsActive
    (`self.AddVolume` ViewVolume)
    (else
      (`self.RemoveVolume` ViewVolume))))

(fn `AddVolume`
  (params (AddedVolume :type "/Game/_GetOutSoldiers/BP/Logic/Camera/Volumes/BP_AViewVolume Object Reference"))
  (bind _addedvolume (`local.AddedVolume`))
  (bind _view (`/Game/_GetOutSoldiers/BP/Logic/Camera/Volumes/BP_AViewVolume.View` _addedvolume))
  (bind _returnvalue (`KismetArrayLibrary.Array_AddUnique` (`self.ActiveViewVolumes`) AddedVolume))
  (if (== _returnvalue -1)
    _
    (elif (not (`BlueprintMapLibrary.Map_Contains` (`self.VolumesPerView`) (`/Game/_GetOutSoldiers/BP/Logic/Camera/Volumes/BP_AViewVolume.View` (`local.AddedVolume`))))
      (`BlueprintMapLibrary.Map_Add` (`self.VolumesPerView`) _view _addedvolume)
      (set `/Game/_GetOutSoldiers/BP/Logic/Camera/Views/BP_AView.bIsActive` true _view))))

(fn `InitViewVolumeBlender`
  (params (ViewVolumes :type "Array of /Game/_GetOutSoldiers/BP/Logic/Camera/Volumes/BP_AViewVolume Object Reference"))
  (locals (NextUId :type Integer))
  (bind _nextuid (`local.NextUId`))
  ;[1 1 1] Init View volumes
  (for _array_element ViewVolumes
    (add `/Game/_GetOutSoldiers/BP/Logic/Camera/Volumes/BP_AViewVolume.ActivationStateUpated` _array_element (`|CreateDelegate` :!event `CE_OnViewVolumeActivationStateUpdated`))
    (`/Game/_GetOutSoldiers/BP/Logic/Camera/Volumes/BP_AViewVolume.InitViewVolume` _array_element _nextuid)
    (`/Engine/EditorBlueprintResources/StandardMacros.IncrementInt` _nextuid)))

(fn `RemoveVolume`
  (params (RemovedVolume :type "/Game/_GetOutSoldiers/BP/Logic/Camera/Volumes/BP_AViewVolume Object Reference"))
  (bind _view (`/Game/_GetOutSoldiers/BP/Logic/Camera/Volumes/BP_AViewVolume.View` (`local.RemovedVolume`)))
  (bind _returnvalue (`KismetArrayLibrary.Array_RemoveItem` (`self.ActiveViewVolumes`) RemovedVolume))
  (if _returnvalue
    (if (`BlueprintMapLibrary.Map_Contains` (`self.VolumesPerView`) _view)
      (`BlueprintMapLibrary.Map_Remove` (`self.VolumesPerView`) _view))))