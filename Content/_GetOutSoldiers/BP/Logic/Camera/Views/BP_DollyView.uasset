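; BP_DollyView is a camera view that follows a target along a rail, like a dolly shot.
; Its GetConfiguration function asks the Rail for a position from the Target's location and uses that as the view location.
; The view rotation is a look-at from that rail point toward the Target, with unit scale.
; Tick and construction only call the parent.
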(event `self.ReceiveTick`
  (params (DeltaSeconds :type "Float (single-precision)"))
  (`parent.ReceiveTick` DeltaSeconds))

(fn `GetConfiguration`
  (returns (ViewConfiguration :type "Transform Structure"))
  (bind _returnvalue (`self.K2_GetActorLocation` (`self.Target`)))
  (bind _railposition (`/Game/_GetOutSoldiers/BP/Logic/Camera/Rail/BP_Rail.GetPosition` (`self.Rail`) _returnvalue))
  (return (`KismetMathLibrary.MakeTransform` _railposition (`KismetMathLibrary.FindLookAtRotation` _railposition _returnvalue))))

(fn `UserConstructionScript`
  (`parent.UserConstructionScript`))