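; BP_ToyCar is a drivable toy car that moves, steers and jumps through Enhanced Input.
; Move input pushes it along control rotation and, when a Box-to-Floor line trace hits, turns the controller by steering times throttle and aligns actor yaw.
; Jump plays a timeline that feeds scaled upward movement input.
; Steering input visually yaws two wheels up to a fixed angle.
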(event `self.ReceiveTick`
  (params (DeltaSeconds :type "Float (single-precision)")))

(event `EnhancedInput|/Game/_GetOutSoldiers/Assets/Inputs/Actions/IA_Move`
  (params (ActionValue :type "Float (double-precision)") (ElapsedSeconds :type "Float (double-precision)") (TriggeredSeconds :type "Float (double-precision)") (InputAction :type "InputAction Object Reference" :default "/Game/_GetOutSoldiers/Assets/Inputs/Actions/IA_Move.IA_Move"))
  (bind (_returnvalue_roll _returnvalue_pitch _returnvalue_yaw) (`KismetMathLibrary.BreakRotator` (`self.GetControlRotation`)))
  (bind (_returnvalue_roll_2 _returnvalue_pitch_2) (`KismetMathLibrary.BreakRotator` (`self.K2_GetActorRotation`)))
  (bind (_returnvalue_roll_3 _returnvalue_pitch_3 _returnvalue_yaw_2) (`KismetMathLibrary.BreakRotator` (`self.GetControlRotation`)))
  (:`Triggered`
    (`self.AddMovementInput` (`KismetMathLibrary.GetForwardVector` (`KismetMathLibrary.MakeRotator` _returnvalue_roll_3 _returnvalue_pitch_3 _returnvalue_yaw_2)) ActionValue)
    (if (`self.Is Grounded`)
      (`self.AddControllerYawInput` (* (`|GetInputActionValue`) (`self.TurnSpeed`) 0.1 ActionValue))
      (`self.K2_SetActorRotation` (`KismetMathLibrary.MakeRotator` _returnvalue_roll_2 _returnvalue_pitch_2 _returnvalue_yaw)))))

(event `EnhancedInput|/Game/_GetOutSoldiers/Assets/Inputs/Actions/IA_Jump`
  (params (ActionValue :type Boolean) (ElapsedSeconds :type "Float (double-precision)") (TriggeredSeconds :type "Float (double-precision)") (InputAction :type "InputAction Object Reference" :default "/Game/_GetOutSoldiers/Assets/Inputs/Actions/IA_Jump.IA_Jump"))
  (:`Started`
    (set `self.IsJumping` true)
    (bind (_direction _jumpscalevalue) (`Timeline|Jump` :!via `PlayFromStart`)
      (:`Update`
        (`self.AddMovementInput` (0.0 0.0 1.0) (* _jumpscalevalue (`self.JumpForce`))))
      (:`Finished`
        (set `self.IsJumping` false)))))

(event `EnhancedInput|/Game/_GetOutSoldiers/Assets/Inputs/Actions/IA_CarSteering`
  (params (ActionValue :type "Float (double-precision)") (ElapsedSeconds :type "Float (double-precision)") (TriggeredSeconds :type "Float (double-precision)") (InputAction :type "InputAction Object Reference" :default "/Game/_GetOutSoldiers/Assets/Inputs/Actions/IA_CarSteering.IA_CarSteering"))
  ;[1 1 1] Rotation des wheels
  (:`Triggered`
    (`SceneComponent.K2_SetRelativeRotation` (`self.Wheel`) (`KismetMathLibrary.MakeRotator` 90.0 0.0 (* (`KismetMathLibrary.SignOfFloat` ActionValue) (`KismetMathLibrary.Lerp` 0.0 20.0 (`KismetMathLibrary.Abs` ActionValue)))) false false :!label _label)
    (`SceneComponent.K2_SetRelativeRotation` (`self.Wheel2`) (`KismetMathLibrary.MakeRotator` 90.0 0.0 (* (`KismetMathLibrary.SignOfFloat` ActionValue) (`KismetMathLibrary.Lerp` 0.0 20.0 (`KismetMathLibrary.Abs` ActionValue)))) false false))
  (:`Completed`
    (goto _label)))

(fn `Is Grounded`
  (returns (ReturnValue :type Boolean))
  (bind (_outhit _returnvalue) (`KismetSystemLibrary.LineTraceSingleByProfile` (`SceneComponent.K2_GetComponentLocation` (`self.Box`)) (`SceneComponent.K2_GetComponentLocation` (`self.Floor`)) "Pawn"))
  (return _returnvalue))

(fn `UserConstructionScript`)