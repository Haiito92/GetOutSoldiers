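; HUD for the Get Out game mode that manages separate UI for a toy car Driver player and a Nounours player.
; On init it creates a hidden end-game menu on the viewport and a canvas on each player's screen, both fed the driver's BP_ToyCar.
; Start, Restart and Leave clicks are relayed through Call functions, while show/hide functions toggle controls, in-game UI and the end-game menu.
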(event `self.ReceiveInitHUD`
  (params (InDriverPlayerController :type "GoSPlayerController Object Reference") (InNoInputPlayerController :type "NoInputPlayerController Object Reference"))
  (bind _asbp_toy_car (cast `/Game/_GetOutSoldiers/BP/Logic/GetOut/Car/BP_ToyCar` (`Controller.K2_GetPawn` InDriverPlayerController))
    (:`then`
      (`self.BP_InitHUD` InDriverPlayerController InNoInputPlayerController _asbp_toy_car))
    (:`CastFailed`
      (`KismetSystemLibrary.PrintString` "BP HUD Get Out : Driver Pawn Cast Failed" true true (struct :`R` 1.0 :`G` 0.020335 :`B` 0.050181 :`A` 1.0)))))

(event `self.ReceiveOnMenuInputActionPressed`
  (params (MenuAction :type "EMenuAction Enum" :default "None"))
  (`KismetSystemLibrary.PrintString` (`|GetEnumeratorNameAsString` MenuAction)))

(event `CE_OnStartButtonClicked`
  ;[1 1 1] React to Controls Menu events
  (`self.StartClicked`))

(event `CE_OnRestartButtonClicked`
  ;[1 1 1] React to End Game Menu events
  (`self.RestartClicked`))

(event `CE_OnLeaveButtonClicked`
  ;[1 1 1] React to End Game Menu events
  (`self.LeaveClicked`))

(fn `BP_InitHUD`
  (params (DriverPlayerController :type "GoSPlayerController Object Reference") (NounoursPlayerController :type "NoInputPlayerController Object Reference") (PlayerPawn :type "/Game/_GetOutSoldiers/BP/Logic/GetOut/Car/BP_ToyCar Object Reference"))
  (bind _wbp_endgamemenu (`self.WBP_EndGameMenu`))
  (`|ExecutionSequence`
    (:`then_1`
      ;[1 1 1] Create EndGame Menu
      (bind _returnvalue (`|CreateWidget` "/Game/_GetOutSoldiers/BP/UI/GetOutLevel/WBP_EndGameMenu.WBP_EndGameMenu_C" (`local.DriverPlayerController`)))
      (bind _output_get (set `self.WBP_EndGameMenu` _returnvalue))
      ;[1 1 1] Bind to End Game Menu events
      (add `/Game/_GetOutSoldiers/BP/UI/GetOutLevel/WBP_EndGameMenu.RestartButtonClicked` _output_get (`|CreateDelegate` :!event `CE_OnRestartButtonClicked`))
      (add `/Game/_GetOutSoldiers/BP/UI/GetOutLevel/WBP_EndGameMenu.LeaveButtonClicked` _output_get (`|CreateDelegate` :!event `CE_OnLeaveButtonClicked`))
      ;[1 1 1] Add to Viewport
      (`Widget.SetVisibility` _wbp_endgamemenu "Hidden")
      (`UserWidget.AddToViewport` _wbp_endgamemenu 0))
    (:`then_2`
      ;[1 1 1] Create Driver Player Canvas
      (bind _returnvalue_2 (`|CreateWidget` "/Game/_GetOutSoldiers/BP/UI/GetOutLevel/Driver/WBP_DriverPlayerCanvas.WBP_DriverPlayerCanvas_C" (`local.DriverPlayerController`)))
      (bind _output_get_2 (set `self.WBP_DriverPlayerCanvas` _returnvalue_2))
      (`/Game/_GetOutSoldiers/BP/UI/GetOutLevel/Driver/WBP_DriverPlayerCanvas.InitDriverCanvas` _output_get_2 (`local.PlayerPawn`))
      (`UserWidget.AddToPlayerScreen` _output_get_2 0)
      (add `/Game/_GetOutSoldiers/BP/UI/GetOutLevel/WBP_ControlsMenu.StartButtonClicked` (`/Game/_GetOutSoldiers/BP/UI/GetOutLevel/Driver/WBP_DriverPlayerCanvas.WBP_ControlsMenu` _output_get_2) (`|CreateDelegate` :!event `CE_OnStartButtonClicked`))
      ;[1 1 1] Create Nounours Player Canvas
      (bind _returnvalue_3 (`|CreateWidget` "/Game/_GetOutSoldiers/BP/UI/GetOutLevel/TeddyBear/WBP_NounoursPlayersCanvas.WBP_NounoursPlayersCanvas_C" (`local.NounoursPlayerController`)))
      (bind _output_get_3 (set `self.WBP_NounoursPlayerCanvas` _returnvalue_3))
      (`/Game/_GetOutSoldiers/BP/UI/GetOutLevel/TeddyBear/WBP_NounoursPlayersCanvas.InitNounoursCanvas` _output_get_3 (`local.PlayerPawn`))
      (`UserWidget.AddToPlayerScreen` _output_get_3 0))))

(fn `HideControls`
  (`/Game/_GetOutSoldiers/BP/UI/GetOutLevel/Driver/WBP_DriverPlayerCanvas.DisplayControls` (`self.WBP_DriverPlayerCanvas`) false)
  (`/Game/_GetOutSoldiers/BP/UI/GetOutLevel/TeddyBear/WBP_NounoursPlayersCanvas.DisplayControls` (`self.WBP_NounoursPlayerCanvas`) false))

(fn `HideEndGameMenu`
  (bind _wbp_endgamemenu (`self.WBP_EndGameMenu`))
  (`/Engine/EditorBlueprintResources/StandardMacros.IsValid` _wbp_endgamemenu
    (:`Is Valid`
      (`Widget.SetVisibility` _wbp_endgamemenu "Hidden"))
    (:`Is Not Valid`
      (`KismetSystemLibrary.PrintString` "End Game Menu Reference Invalid" true true (struct :`R` 1.0 :`G` 0.597625 :`A` 1.0)))))

(fn `HideInGameUI`
  (`/Game/_GetOutSoldiers/BP/UI/GetOutLevel/Driver/WBP_DriverPlayerCanvas.DisplayInGameUI` (`self.WBP_DriverPlayerCanvas`) false)
  (`/Game/_GetOutSoldiers/BP/UI/GetOutLevel/TeddyBear/WBP_NounoursPlayersCanvas.DisplayInGameUI` (`self.WBP_NounoursPlayerCanvas`) false))

(fn `ShowControls`
  (`/Game/_GetOutSoldiers/BP/UI/GetOutLevel/Driver/WBP_DriverPlayerCanvas.DisplayControls` (`self.WBP_DriverPlayerCanvas`) true)
  (`/Game/_GetOutSoldiers/BP/UI/GetOutLevel/TeddyBear/WBP_NounoursPlayersCanvas.DisplayControls` (`self.WBP_NounoursPlayerCanvas`) true))

(fn `ShowEndGameMenu`
  (bind _wbp_endgamemenu (`self.WBP_EndGameMenu`))
  (`/Engine/EditorBlueprintResources/StandardMacros.IsValid` _wbp_endgamemenu
    (:`Is Valid`
      (`Widget.SetVisibility` _wbp_endgamemenu "Visible"))
    (:`Is Not Valid`
      (`KismetSystemLibrary.PrintString` "End Game Menu Reference Invalid" true true (struct :`R` 1.0 :`G` 0.597625 :`A` 1.0)))))

(fn `ShowInGameUI`
  (`/Game/_GetOutSoldiers/BP/UI/GetOutLevel/Driver/WBP_DriverPlayerCanvas.DisplayInGameUI` (`self.WBP_DriverPlayerCanvas`) true)
  (`/Game/_GetOutSoldiers/BP/UI/GetOutLevel/TeddyBear/WBP_NounoursPlayersCanvas.DisplayInGameUI` (`self.WBP_NounoursPlayerCanvas`) true))

(fn `UserConstructionScript`)