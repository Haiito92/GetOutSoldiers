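; PC_GetOut is the player controller for the GetOut game, managing Enhanced Input contexts for menu and gameplay.
; On init it requests Menu mode through CE_SetInputMode, which swaps the menu mapping context against the car and teddy bear contexts.
; Pressing IA_Interact fires OnStartGamePressed, leaving the response and any switch to Gameplay mode to code outside this controller.
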(event `InitPlayerController`
  (`self.CE_SetInputMode` "NewEnumerator1"))

(event `CE_SetInputMode`
  (params (InputMode :type "/Game/_GetOutSoldiers/BP/Logic/GetOut/EN_InputMode Enum" :default "NewEnumerator0"))
  (bind _returnvalue (subsystem `EnhancedInputLocalPlayerSubsystem`))
  ;[0 0.1082 0.3781] InputMode
  (switch `/Game/_GetOutSoldiers/BP/Logic/GetOut/EN_InputMode` InputMode
    (:`NewEnumerator0`
      (`EnhancedInputSubsystemInterface.RemoveMappingContext` _returnvalue "/Game/_GetOutSoldiers/Assets/Inputs/IMC_Menu.IMC_Menu" (struct))
      (`EnhancedInputSubsystemInterface.AddMappingContext` _returnvalue "/Game/_GetOutSoldiers/Assets/Inputs/IMC_Car.IMC_Car" 0 (struct))
      (`EnhancedInputSubsystemInterface.AddMappingContext` _returnvalue "/Game/_GetOutSoldiers/Assets/Inputs/IMC_TeddyBear.IMC_TeddyBear" 0 (struct)))
    (:`NewEnumerator1`
      (`EnhancedInputSubsystemInterface.RemoveMappingContext` _returnvalue "/Game/_GetOutSoldiers/Assets/Inputs/IMC_TeddyBear.IMC_TeddyBear" (struct))
      (`EnhancedInputSubsystemInterface.RemoveMappingContext` _returnvalue "/Game/_GetOutSoldiers/Assets/Inputs/IMC_Car.IMC_Car" (struct))
      (`EnhancedInputSubsystemInterface.AddMappingContext` _returnvalue "/Game/_GetOutSoldiers/Assets/Inputs/IMC_Menu.IMC_Menu" 0 (struct)))))

(event `EnhancedInput|/Game/_GetOutSoldiers/Assets/Inputs/Actions/IA_Interact`
  (params (ActionValue :type Boolean) (ElapsedSeconds :type "Float (double-precision)") (TriggeredSeconds :type "Float (double-precision)") (InputAction :type "InputAction Object Reference" :default "/Game/_GetOutSoldiers/Assets/Inputs/Actions/IA_Interact.IA_Interact"))
  (:`Started`
    (`self.OnStartGamePressed`)))

(fn `UserConstructionScript`)