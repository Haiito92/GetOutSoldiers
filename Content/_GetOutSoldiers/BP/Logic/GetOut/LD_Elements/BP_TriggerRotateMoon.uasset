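; Trigger actor that starts the moons rotating when the toy car drives into its box.
; The first BP_ToyCar overlap calls StartRotation on every BP_Moon in the level, then destroys the trigger.
; BeginPlay still creates an LS_Moon sequence player, but its looping playback and a StartTurningMoon call are left disconnected.
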(event `self.ReceiveBeginPlay`
  (bind (_outactor _returnvalue) (`LevelSequencePlayer.CreateLevelSequencePlayer` "/Game/_GetOutSoldiers/Assets/Level_Sequence/LS_Moon.LS_Moon"))
  (set `self.RotateMoon` _returnvalue))

(event `self.Box.OnComponentBeginOverlap`
  (params (OverlappedComponent :type "PrimitiveComponent Object Reference") (OtherActor :type "Actor Object Reference") (OtherComp :type "PrimitiveComponent Object Reference") (OtherBodyIndex :type Integer) (bFromSweep :type Boolean) (SweepResult :type "HitResult Structure (by ref)"))
  (cast `/Game/_GetOutSoldiers/BP/Logic/GetOut/Car/BP_ToyCar` OtherActor)
  (`/Engine/EditorBlueprintResources/StandardMacros.DoOnce` false
    (:`Completed`
      (bind _outactors (`GameplayStatics.GetAllActorsOfClass` "/Game/_GetOutSoldiers/BP/Logic/GetOut/LD_Elements/BP_Moon.BP_Moon_C"))
      (for _array_element _outactors
        (`/Game/_GetOutSoldiers/BP/Logic/GetOut/LD_Elements/BP_Moon.StartRotation` _array_element))
      (`self.K2_DestroyActor`))))

(fn `UserConstructionScript`)