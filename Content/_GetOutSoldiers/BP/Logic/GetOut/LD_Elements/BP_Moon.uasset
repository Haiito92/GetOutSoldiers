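; BP_Moon is a level-design moon actor that spins continuously once its StartRotation event is called.
; A timeline lerps the actor's yaw through a full turn from its current rotation, then calls StartRotation again on finish to loop.
; BeginPlay is inactive, so nothing in this Blueprint starts the spin.
; An older half-turn rotation of the Cube component is left disconnected, and its StartTurningMoon event is empty.
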(event `StartTurningMoon`)

(event `StartRotation`
  (bind (_rotation_roll _rotation_pitch _rotation_yaw) (`KismetMathLibrary.BreakRotator` (`self.Rotation`)))
  (set `self.Rotation` (`self.K2_GetActorRotation`))
  (bind (_direction _newtrack_0) (`Timeline|Rotate` :!via `PlayFromStart`)
    (:`Update`
      (`self.K2_SetActorRotation` (`KismetMathLibrary.RLerp` (`self.Rotation`) (`KismetMathLibrary.MakeRotator` _rotation_roll _rotation_pitch (+ _rotation_yaw 360.0)) _newtrack_0)))
    (:`Finished`
      (`self.StartRotation`))))

(fn `UserConstructionScript`)