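; Component that turns teddy bear button inputs, such as movement, jump and voice commands, into 2D sounds.
; Each input looks up its row in DT_TeddyBear_Buttons, plays the sound and fires OnSoundPlayed with the row's value and notification.
; It records the last action and its timestamp, so a row's special sound replaces the default when it follows a specific action within a time window.
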(event `EnhancedInput|/Game/_GetOutSoldiers/Assets/Inputs/Actions/TeddyBear/IA_Teddy_Backward`
  (params (ActionValue :type Boolean) (ElapsedSeconds :type "Float (double-precision)") (TriggeredSeconds :type "Float (double-precision)") (InputAction :type "InputAction Object Reference" :default "/Game/_GetOutSoldiers/Assets/Inputs/Actions/TeddyBear/IA_Teddy_Backward.IA_Teddy_Backward"))
  ;[1 1 1] Comment
  (:`Started`
    (`self.PlayTeddyBearSound` "Backward")))

(event `EnhancedInput|/Game/_GetOutSoldiers/Assets/Inputs/Actions/TeddyBear/IA_Teddy_Left`
  (params (ActionValue :type Boolean) (ElapsedSeconds :type "Float (double-precision)") (TriggeredSeconds :type "Float (double-precision)") (InputAction :type "InputAction Object Reference" :default "/Game/_GetOutSoldiers/Assets/Inputs/Actions/TeddyBear/IA_Teddy_Left.IA_Teddy_Left"))
  ;[1 1 1] Comment
  (:`Started`
    (`self.PlayTeddyBearSound` "Left")))

(event `EnhancedInput|/Game/_GetOutSoldiers/Assets/Inputs/Actions/TeddyBear/IA_Teddy_Forward`
  (params (ActionValue :type Boolean) (ElapsedSeconds :type "Float (double-precision)") (TriggeredSeconds :type "Float (double-precision)") (InputAction :type "InputAction Object Reference" :default "/Game/_GetOutSoldiers/Assets/Inputs/Actions/TeddyBear/IA_Teddy_Forward.IA_Teddy_Forward"))
  ;[1 1 1] Comment
  (:`Started`
    (`self.PlayTeddyBearSound` "Forward")))

(event `EnhancedInput|/Game/_GetOutSoldiers/Assets/Inputs/Actions/TeddyBear/IA_Teddy_Right`
  (params (ActionValue :type Boolean) (ElapsedSeconds :type "Float (double-precision)") (TriggeredSeconds :type "Float (double-precision)") (InputAction :type "InputAction Object Reference" :default "/Game/_GetOutSoldiers/Assets/Inputs/Actions/TeddyBear/IA_Teddy_Right.IA_Teddy_Right"))
  ;[1 1 1] Comment
  (:`Started`
    (`self.PlayTeddyBearSound` "Right")))

(event `EnhancedInput|/Game/_GetOutSoldiers/Assets/Inputs/Actions/TeddyBear/IA_Teddy_Jump`
  (params (ActionValue :type Boolean) (ElapsedSeconds :type "Float (double-precision)") (TriggeredSeconds :type "Float (double-precision)") (InputAction :type "InputAction Object Reference" :default "/Game/_GetOutSoldiers/Assets/Inputs/Actions/TeddyBear/IA_Teddy_Jump.IA_Teddy_Jump"))
  ;[1 1 1] Comment
  (:`Started`
    (`self.PlayTeddyBearSound` "Jump")))

(event `EnhancedInput|/Game/_GetOutSoldiers/Assets/Inputs/Actions/TeddyBear/IA_Teddy_Stop`
  (params (ActionValue :type Boolean) (ElapsedSeconds :type "Float (double-precision)") (TriggeredSeconds :type "Float (double-precision)") (InputAction :type "InputAction Object Reference" :default "/Game/_GetOutSoldiers/Assets/Inputs/Actions/TeddyBear/IA_Teddy_Stop.IA_Teddy_Stop"))
  ;[1 1 1] Other Commands
  (:`Started`
    (`self.PlayTeddyBearSound` "Stop")))

(event `EnhancedInput|/Game/_GetOutSoldiers/Assets/Inputs/Actions/TeddyBear/IA_Teddy_Looser`
  (params (ActionValue :type Boolean) (ElapsedSeconds :type "Float (double-precision)") (TriggeredSeconds :type "Float (double-precision)") (InputAction :type "InputAction Object Reference" :default "/Game/_GetOutSoldiers/Assets/Inputs/Actions/TeddyBear/IA_Teddy_Looser.IA_Teddy_Looser"))
  ;[1 1 1] Other Commands
  (:`Started`
    (`self.PlayTeddyBearSound` "Looser")))

(event `EnhancedInput|/Game/_GetOutSoldiers/Assets/Inputs/Actions/TeddyBear/IA_Teddy_Youpi`
  (params (ActionValue :type Boolean) (ElapsedSeconds :type "Float (double-precision)") (TriggeredSeconds :type "Float (double-precision)") (InputAction :type "InputAction Object Reference" :default "/Game/_GetOutSoldiers/Assets/Inputs/Actions/TeddyBear/IA_Teddy_Youpi.IA_Teddy_Youpi"))
  ;[1 1 1] Other Commands
  (:`Started`
    (`self.PlayTeddyBearSound` "Youpi")))

(fn `GetSpecialSound`
  (params (PossibleSpecialSounds :type "Array of /Game/_GetOutSoldiers/BP/Logic/GetOut/TeddyBear/ST_TBSpecialSounds Structure"))
  (returns (Found :type Boolean) (Sound :type "SoundBase Object Reference"))
  (for _array_element PossibleSpecialSounds
    (if (`self.ShouldPlaySpecialSound` _array_element)
      (return true (`.SpecialSound_11_D02EC4ED45B2B30481DF6E85DCB2B887` (break `/Game/_GetOutSoldiers/BP/Logic/GetOut/TeddyBear/ST_TBSpecialSounds` _array_element)))))
  (return false null))

(fn `PlayTeddyBearSound`
  (params (Action :type Name))
  (bind _returnvalue (`|GetDataTableRow` "/Game/_GetOutSoldiers/Assets/Data/DT_TeddyBear_Buttons.DT_TeddyBear_Buttons" Action)
    (:`then`
      (bind (_found _sound) (`self.GetSpecialSound` (`.SpecialSounds_9_8145C0E8460B2024C76CBA9B2947284C` (break `/Game/_GetOutSoldiers/BP/Logic/GetOut/TeddyBear/ST_TeddyBear` _returnvalue))))
      (`GameplayStatics.PlaySound2D` (select `bool` _found :`false` (`.Sound_2_1E80984E4449643589866AB8B3F807FE` (break `/Game/_GetOutSoldiers/BP/Logic/GetOut/TeddyBear/ST_TeddyBear` _returnvalue)) :`true` _sound) 1.0 1.0 0.0 null null)
      (`self.OnSoundPlayed` (break `/Game/_GetOutSoldiers/BP/Logic/GetOut/TeddyBear/ST_TeddyBear` _returnvalue) (`.Notification_12_63217F294A36E0F09B654B92702A65D8` (break `/Game/_GetOutSoldiers/BP/Logic/GetOut/TeddyBear/ST_TeddyBear` _returnvalue)))
      (set `self.PreviousAction` (break `/Game/_GetOutSoldiers/BP/Logic/GetOut/TeddyBear/ST_TeddyBear` _returnvalue))
      (set `self.TimeSincePreviousAction` (`GameplayStatics.GetTimeSeconds`)))))

(fn `ShouldPlaySpecialSound`
  (params (SpecialSound :type "/Game/_GetOutSoldiers/BP/Logic/GetOut/TeddyBear/ST_TBSpecialSounds Structure"))
  (returns (ShouldPlay :type Boolean))
  (return (and (`|EnumEquality` (`self.PreviousAction`) SpecialSound_PreviousActionPlayed_10_E13D80D34CB9CEFABF555B88F41F639B) (> (+ (`self.TimeSincePreviousAction`) SpecialSound_Time_9_37A76B0E4CFFB86B5FC2329E2CB929CE) (`GameplayStatics.GetTimeSeconds`)))))