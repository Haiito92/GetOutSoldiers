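; Game mode for the GetOut level, where the player drives a toy car, running a three-phase flow from waiting through play to game over.
; On BeginPlay it caches the game instance, player controller, car and HUD, binds their events and starts the camera world subsystem.
; Start input hides the controls and switches input mode; the player death event shows the end menu.
; Restart and Leave load levels through the game instance, while pause functions are empty.
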(event `self.ReceiveBeginPlay`
  (`|ExecutionSequence`
    (:`then_0`
      ;[1 1 1] Get GI
      (bind _asgi_get_out_soldiers (cast `/Game/_GetOutSoldiers/BP/Logic/GI_GetOutSoldiers` (`GameplayStatics.GetGameInstance`))
        (:`then`
          (set `self.GameInstance` _asgi_get_out_soldiers)
          (`self.InitGame`))
        (:`CastFailed`
          (`KismetSystemLibrary.PrintString` "Couldn't get GI_GetOutSoldiers" true true (struct :`R` 1.0 :`G` 0.017487 :`A` 1.0) 2.0 "None"))))
    (:`then_1`
      (`/Game/_GetOutSoldiers/BP/Logic/GetOut/HUD_GetOut.ShowControls` (`self.HUD_GetOut`)))))

(event `CE_OnStartClicked`
  (if (`|EnumEquality` (`self.GamePhase`) "NewEnumerator0")
    (`self.StartGame`)))

(event `CE_OnHUDRestartClicked`
  ;[1 1 1] React to HUD Events
  (`self.Restart`))

(event `CE_OnHUDLeaveClicked`
  ;[1 1 1] React to HUD Events
  (`self.Leave`))

(event `CE_OnPlayerDeath`
  ;[1 1 1] Player Death
  (`self.EndGame`))

(fn `EndGame`
  (set `self.GamePhase` "NewEnumerator2")
  (`/Game/_GetOutSoldiers/BP/Logic/GetOut/HUD_GetOut.ShowEndGameMenu` (`self.HUD_GetOut`))
  (`/Game/_GetOutSoldiers/BP/Logic/GetOut/PC_GetOut.CE_SetInputMode` (`self.PC Get Out`) "NewEnumerator1"))

(fn `InitGame`
  (bind _returnvalue (subsystem `CameraWorldSubsystem`))
  (bind _hud_getout (`self.HUD_GetOut`))
  (`|ExecutionSequence`
    (:`then_0`
      (set `self.GamePhase` "NewEnumerator0")
      ;[1 1 1] Init Logic
      (bind _aspc_get_out (cast `/Game/_GetOutSoldiers/BP/Logic/GetOut/PC_GetOut` (`GameplayStatics.GetPlayerController` 0)))
      (bind _output_get (set `self.PC Get Out` _aspc_get_out))
      (`/Game/_GetOutSoldiers/BP/Logic/GetOut/PC_GetOut.InitPlayerController` _output_get)
      (add `/Game/_GetOutSoldiers/BP/Logic/GetOut/PC_GetOut.OnStartGamePressed` _output_get (`|CreateDelegate` :!event `CE_OnStartClicked`))
      (bind _asbp_toy_car (cast `/Game/_GetOutSoldiers/BP/Logic/GetOut/Car/BP_ToyCar` (`GameplayStatics.GetPlayerPawn` 0)))
      (set `self.Player` _asbp_toy_car)
      ;[1 1 1] Init HUD
      (bind _ashud_get_out (cast `/Game/_GetOutSoldiers/BP/Logic/GetOut/HUD_GetOut` (`PlayerController.GetHUD` _output_get))
        (:`then`
          (bind _output_get_2 (set `self.HUD_GetOut` _ashud_get_out))
          (`/Game/_GetOutSoldiers/BP/Logic/GetOut/HUD_GetOut.InitHUD` _output_get_2 (`self.PC Get Out`))
          ;[1 1 1] Bind to HUD events
          (add `/Game/_GetOutSoldiers/BP/Logic/GetOut/HUD_GetOut.StartClicked` _hud_getout (`|CreateDelegate` :!event `CE_OnStartClicked`))
          (add `/Game/_GetOutSoldiers/BP/Logic/GetOut/HUD_GetOut.RestartClicked` _hud_getout (`|CreateDelegate` :!event `CE_OnHUDRestartClicked`))
          (add `/Game/_GetOutSoldiers/BP/Logic/GetOut/HUD_GetOut.LeaveClicked` _hud_getout (`|CreateDelegate` :!event `CE_OnHUDLeaveClicked`)))
        (:`CastFailed`
          (`KismetSystemLibrary.PrintString` "Couldn't get HUDGetOut" true true (struct :`R` 1.0 :`G` 0.017487 :`A` 1.0) 2.0 "None"))))
    (:`then_1`
      (`CameraWorldSubsystem.InitializeCameraWorldSubsystem` _returnvalue)
      (`CameraWorldSubsystem.StartCameraWorldSubsystem` _returnvalue))))

(fn `Leave`
  (`/Game/_GetOutSoldiers/BP/Logic/GI_GetOutSoldiers.LoadLevel` (`self.GameInstance`) "Level_MainMenu"))

(fn `PauseGame`)

(fn `Restart`
  (`/Game/_GetOutSoldiers/BP/Logic/GI_GetOutSoldiers.LoadLevel` (`self.GameInstance`) "Level_GetOut"))

(fn `StartGame`
  (`/Game/_GetOutSoldiers/BP/Logic/GetOut/HUD_GetOut.HideControls` (`self.HUD_GetOut`))
  (`/Game/_GetOutSoldiers/BP/Logic/GetOut/PC_GetOut.CE_SetInputMode` (`self.PC Get Out`) "NewEnumerator0")
  (set `self.GamePhase` "NewEnumerator1"))

(fn `UnpauseGame`)

(fn `UserConstructionScript`)